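; BP_Ranger is an AI-moved pawn that patrols a looping route of path points.
; On BeginPlay it finds BP_PathManager in the level, picks its first destination and enters the Patrol state.
; Tick switches on State and issues AIMoveTo while patrolling; each success advances through the manager's Path array, wrapping at the end.
; Only the Patrol state has logic here.
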(event `self.ReceiveBeginPlay`
  (bind _returnvalue (`GameplayStatics.GetActorOfClass` "/Game/PatrolAndChaseExample/BP_PathManager.BP_PathManager_C"))
  (set `self.pathManager` _returnvalue)
  (`self.UpdateDestination`)
  (set `self.state` "NewEnumerator0"))

(event `self.ReceiveTick`
  (params (DeltaSeconds :type "Float (single-precision)"))
  (switch `/Game/PatrolAndChaseExample/ERangerState` (`self.state`)
    (:`NewEnumerator0`
      (`|AIMoveTo` self (`self.destination`) null 2.0
        (:`OnSuccess`
          (`self.UpdateDestination`))))))

(fn `UpdateDestination`
  (bind _index (`self.index`))
  (set `self.destination` (`self.K2_GetActorLocation` (`|GetArrayItem` (`/Game/PatrolAndChaseExample/BP_PathManager.path` (`self.pathManager`)) _index)))
  (bind _result (`/Engine/EditorBlueprintResources/StandardMacros.IncrementInt` _index)
    (:`  `
      (if (>= _result (`KismetArrayLibrary.Array_Length` (`/Game/PatrolAndChaseExample/BP_PathManager.path` (`self.pathManager`))))
        (set `self.index` 0)))))

(fn `UserConstructionScript`)