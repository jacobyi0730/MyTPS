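; Third-person player character in a patrol-and-chase example, handling movement, mouse look and jumping.
; Tick reads both movement axes, rotates them by the player controller's transform, flattens and normalizes the result, then feeds it to movement input.
; Rifle and bullet firing, hit-scan impulses, camera shake, walk/idle animation, crosshair, sniper zoom and gun switching remain as disconnected nodes that never run.
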(event `self.ReceiveBeginPlay`)

(event `InputAction|ChooseGun` :overrideparent false
  (params (Key :type "Key Structure")))

(event `InputAxis|Move Forward / Backward` :overrideparent false
  (params (AxisValue :type "Float (single-precision)")))

(event `InputAction|ChooseSniperGun` :overrideparent false
  (params (Key :type "Key Structure")))

(event `InputAction|Zoom` :overrideparent false
  (params (Key :type "Key Structure")))

(event `InputAction|Fire` :overrideparent false
  (params (Key :type "Key Structure")))

(event `self.ReceiveTick`
  (params (DeltaSeconds :type "Float (single-precision)"))
  (bind (_returnvalue_x _returnvalue_y) (`KismetMathLibrary.BreakVector` (`KismetMathLibrary.TransformDirection` (`self.GetTransform` (`GameplayStatics.GetPlayerController` 0)) (`KismetMathLibrary.MakeVector` (`self.GetInputAxisValue`) (`self.GetInputAxisValue`)))))
  (`self.AddMovementInput` (`KismetMathLibrary.Normal` (`KismetMathLibrary.MakeVector` _returnvalue_x _returnvalue_y))))

(event `InputAxis|Look Up / Down Mouse` :overrideparent false
  (params (AxisValue :type "Float (single-precision)"))
  (`self.AddControllerPitchInput` AxisValue))

(event `InputAxis|Turn Right / Left Mouse` :overrideparent false
  (params (AxisValue :type "Float (single-precision)"))
  (`self.AddControllerYawInput` AxisValue))

(event `InputAction|Jump` :overrideparent false
  (params (Key :type "Key Structure"))
  (:`Pressed`
    (`self.Jump`)))

(fn `UserConstructionScript`)