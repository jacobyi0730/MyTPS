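; Enemy character that patrols, chases, attacks and reacts to damage through a state machine evaluated on Tick.
; Patrol loops through path manager waypoints with AIMoveTo; AI perception of the player within detect range starts a chase, which leads to timed attacks toggled on its AnimBP.
; Distance checks drop it back to chase or patrol.
; Damage plays random hit montages; death disables collision, then sinks the body once TryRealDie flags completion.
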(event `self.AIPerception.OnPerceptionUpdated`
  (params (UpdatedActors :type "Array of Actor Object Reference (by ref)"))
  (switch `/Game/PatrolAndChaseExample/ERangerState` (`self.state`)
    (:`NewEnumerator0`
      (if (> (`KismetArrayLibrary.Array_Length` UpdatedActors) 0)
        (cast `/Game/PatrolAndChaseExample/BP_NewTPSPlayer` (`|GetArrayItem` UpdatedActors))
        (bind _distance (`self.GetDistance`))
        (if (< _distance (`self.detectDistance`))
          (set `self.state` "NewEnumerator1"))))))

(event `self.ReceiveBeginPlay`
  (bind _returnvalue (`GameplayStatics.GetActorOfClass` "/Game/PatrolAndChaseExample/BP_PathManager.BP_PathManager_C"))
  (set `self.pathManager` _returnvalue)
  (`self.UpdateDestination`)
  (set `self.state` "NewEnumerator0")
  (set `self.hp` (`self.maxHP`)))

(event `self.ReceiveTick`
  (params (DeltaSeconds :type "Float (single-precision)"))
  (switch `/Game/PatrolAndChaseExample/ERangerState` (`self.state`)
    (:`NewEnumerator0`
      ;[1 1 1] Patrol
      (`|AIMoveTo` self (`self.destination`) null 2.0
        (:`OnSuccess`
          (`self.UpdateDestination`))))
    (:`NewEnumerator1`
      ;[1 1 1] Chase
      (`|AIMoveTo` self (`self.K2_GetActorLocation` (`GameplayStatics.GetPlayerPawn` 0)) null 160.0
        (:`then`
          (bind _distance (`self.GetDistance`))
          (if (> _distance (`self.chaseDistance`))
            (set `self.state` "NewEnumerator0")))
        (:`OnSuccess`
          (set `self.state` "NewEnumerator4"))))
    (:`NewEnumerator4`
      ;[1 1 1] Attack
      (bind _output_get (set `self.curTime` (+ (`self.curTime`) (`GameplayStatics.GetWorldDeltaSeconds`))))
      (if (> _output_get (`self.attackWaitDelay`))
        (bind _distance_2 (`self.GetDistance`))
        (if (>= _distance_2 (`self.attackDistance`))
          (set `self.state` "NewEnumerator1")
          (set `/Game/PatrolAndChaseExample/ABP_NewEnemy.bAttackPlay` false (stale _asabp_new_enemy))
          (set `self.curTime` 0.0)
          (else
            (bind _asabp_new_enemy (cast `/Game/PatrolAndChaseExample/ABP_NewEnemy` (`SkeletalMeshComponent.GetAnimInstance` (`self.Mesh`))))
            (set `/Game/PatrolAndChaseExample/ABP_NewEnemy.bAttackPlay` true _asabp_new_enemy)
            (set `self.curTime` 0.0)))))
    (:`NewEnumerator6`
      ;[1 1 1] Die
      (if (`self.bDieAnimDone`)
        (`self.K2_SetActorLocation` (+ (`self.K2_GetActorLocation`) (* (`KismetMathLibrary.Vector_Down`) 100.0 (`GameplayStatics.GetWorldDeltaSeconds`))))))))

(fn `DoDamage`
  (set `self.state` "NewEnumerator5")
  (`Controller.StopMovement` (`self.GetController`))
  (`self.PlayAnimMontage` "/Game/PatrolAndChaseExample/NewEnemyMontage.NewEnemyMontage" 1.0 (`KismetStringLibrary.Conv_StringToName` (`KismetStringLibrary.Concat_StrStr` "Damage" (`KismetStringLibrary.Conv_IntToString` (`KismetMathLibrary.RandomIntegerInRange` 0 1))))))

(fn `DoDie`
  (set `self.state` "NewEnumerator6")
  (`Controller.StopMovement` (`self.GetController`))
  (`PrimitiveComponent.SetCollisionEnabled` (`self.CapsuleComponent`) "NoCollision")
  (`self.PlayAnimMontage` "/Game/PatrolAndChaseExample/NewEnemyMontage.NewEnemyMontage" 1.0 "Die")
  (set `self.bDieAnimDone` false))

(fn `GetDistance`
  (returns (distance :type "Float (double-precision)"))
  (return (`KismetMathLibrary.Vector_Distance` (`self.K2_GetActorLocation`) (`self.K2_GetActorLocation` (`GameplayStatics.GetPlayerPawn` 0)))))

(fn `OnMyDamageProcess`
  (params (damage :type Integer))
  (bind _output_get (set `self.hp` (- (`self.hp`) damage)))
  (if (> _output_get 0)
    (`self.DoDamage`)
    (else
      (`self.DoDie`))))

(fn `TryRealDie`
  (set `self.bDieAnimDone` true)
  (`self.SetLifeSpan` 2.0))

(fn `UpdateDestination`
  (bind _index (`self.index`))
  (set `self.destination` (`self.K2_GetActorLocation` (`|GetArrayItem` (`/Game/PatrolAndChaseExample/BP_PathManager.path` (`self.pathManager`)) _index)))
  (bind _result (`/Engine/EditorBlueprintResources/StandardMacros.IncrementInt` _index)
    (:`  `
      (if (>= _result (`KismetArrayLibrary.Array_Length` (`/Game/PatrolAndChaseExample/BP_PathManager.path` (`self.pathManager`))))
        (set `self.index` 0)))))

(fn `UserConstructionScript`)