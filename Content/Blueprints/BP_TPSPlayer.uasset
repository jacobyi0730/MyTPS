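; Third-person shooter player Blueprint whose event graph logic is almost entirely disconnected, with empty input and lifecycle events.
; The unreachable fragments cover camera-relative movement, look, jump, bullet spawning, line-trace shots with explosion and physics impulse, and fire montage with sound and camera shake.
; Other orphaned fragments handle crosshair and sniper-zoom widgets, FOV changes and walk/idle animation.
; SetGun toggles rifle and sniper mesh visibility, but only orphaned nodes call it here.
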(event `self.ReceiveBeginPlay`)

(event `InputAction|ChooseGun` :overrideparent false
  (params (Key :type "Key Structure")))

(event `InputAxis|Move Forward / Backward` :overrideparent false
  (params (AxisValue :type "Float (single-precision)")))

(event `InputAction|ChooseSniperGun` :overrideparent false
  (params (Key :type "Key Structure")))

(event `InputAction|Zoom` :overrideparent false
  (params (Key :type "Key Structure")))

(event `InputAction|Fire` :overrideparent false
  (params (Key :type "Key Structure")))

(event `self.ReceiveTick`
  (params (DeltaSeconds :type "Float (single-precision)")))

(event `InputAxis|Look Up / Down Mouse` :overrideparent false
  (params (AxisValue :type "Float (single-precision)")))

(event `InputAxis|Turn Right / Left Mouse` :overrideparent false
  (params (AxisValue :type "Float (single-precision)")))

(event `InputAction|Jump` :overrideparent false
  (params (Key :type "Key Structure")))

(fn `Set Gun`
  (params (isSniperGun :type Boolean))
  (`SceneComponent.SetVisibility` (`self.sniperMeshComp`) isSniperGun false)
  (`SceneComponent.SetVisibility` (`self.gunMeshComp`) (not isSniperGun) false))

(fn `UserConstructionScript`)