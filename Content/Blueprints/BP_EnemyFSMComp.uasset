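; BP_EnemyFSMComp is an actor component that drives BP_Enemy behavior with a simple state machine.
; Tick switches on EnemyState: Idle acquires the TPSPlayer after a delay, then Move steps straight toward it without sweep until within AttackDistance.
; Attack only prints after a delay, returning to Move when the player leaves range.
; Damage passes straight to Die, which destroys the enemy; nothing here triggers Damage.
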(event `self.ReceiveBeginPlay`
  ;[1 1 1] 태어날 때
  (bind _asbp_enemy (cast `/Game/Blueprints/BP_Enemy` (`self.GetOwner`)))
  (set `self.enemy` _asbp_enemy)
  (set `self.enemyState` "NewEnumerator0"))

(event `self.ReceiveTick`
  (params (DeltaSeconds :type "Float (single-precision)"))
  (bind _enemy (`self.enemy`))
  (switch `/Game/Blueprints/EEnemyFSMState` (`self.enemyState`)
    (:`NewEnumerator0`
      ;[1 1 1] Idle
      (`KismetSystemLibrary.Delay` 0.5)
      (bind _astpsplayer (cast `TPSPlayer` (`GameplayStatics.GetPlayerPawn` 0)))
      (set `self.target` _astpsplayer)
      (set `self.enemyState` "NewEnumerator1"))
    (:`NewEnumerator1`
      ;[1 1 1] Move
      (`Actor.K2_SetActorLocation` _enemy (+ (`Actor.K2_GetActorLocation` _enemy) (* (`KismetMathLibrary.Normal` (- (`Actor.K2_GetActorLocation` (`self.target`)) (`Actor.K2_GetActorLocation` (`self.enemy`)))) (`self.speed`) (`GameplayStatics.GetWorldDeltaSeconds`))) false false)
      (if (< (`KismetMathLibrary.Vector_Distance` (`Actor.K2_GetActorLocation` (`self.target`)) (`Actor.K2_GetActorLocation` (`self.enemy`))) (`self.attackDistance`))
        (set `self.enemyState` "NewEnumerator2")))
    (:`NewEnumerator2`
      ;[1 1 1] Attack
      (`KismetSystemLibrary.Delay` 1.0)
      (`KismetSystemLibrary.PrintString` "Attack")
      (if (>= (`KismetMathLibrary.Vector_Distance` (`Actor.K2_GetActorLocation` (`self.target`)) (`Actor.K2_GetActorLocation` (`self.enemy`))) (`self.attackDistance`))
        (set `self.enemyState` "NewEnumerator1")))
    (:`NewEnumerator3`
      (set `self.enemyState` "NewEnumerator4"))
    (:`NewEnumerator4`
      (`Actor.K2_DestroyActor` (`self.enemy`)))))